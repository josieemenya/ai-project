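; Spline-driven wall actor that tiles a target mesh along its spline, deformed to follow the curve.
; The construction script destroys existing spline mesh components, then adds one Movable segment per whole MeshLength of spline.
; Each segment takes local positions and unscaled tangents sampled by distance at its two ends.
; Any leftover shorter than MeshLength stays uncovered, and the event graph has no active logic.
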(fn `GenerateSplineMesh`
  (bind _meshlength (`self.MeshLength`))
  (bind _spline (`self.Spline`))
  (bind _spline_2 (`self.Spline`))
  (bind _returnvalue (`KismetMathLibrary.FTrunc` (/ (`SplineComponent.GetSplineLength` (`self.Spline`)) _meshlength)))
  (for _array_element (`self.K2_GetComponentsByClass` "/Script/Engine.SplineMeshComponent")
    (`ActorComponent.K2_DestroyComponent` _array_element))
  (if (> _returnvalue 0)
    (bind _result (`/Engine/EditorBlueprintResources/StandardMacros.DecrementInt` _returnvalue)
      (:`  `
        (for _index (range (+ _result 1))
          (bind _returnvalue_2 (`AddComponent|NODE_AddSplineMeshComponent-0`))
          (`SceneComponent.SetMobility` _returnvalue_2 "Movable")
          (`SceneComponent.K2_AttachToComponent` _returnvalue_2 (`self.Spline`) "None" "KeepRelative" "KeepRelative" "KeepRelative" true)
          (`StaticMeshComponent.SetStaticMesh` _returnvalue_2 (`self.TargetMesh`))
          (bind _returnvalue_3 (* _index _meshlength))
          (bind _returnvalue_4 (* (`self.MeshLength`) (+ _index 1)))
          (`SplineMeshComponent.SetStartAndEnd` _returnvalue_2 (`SplineComponent.GetLocationAtDistanceAlongSpline` _spline_2 _returnvalue_3 "Local") (`SplineComponent.GetTangentAtDistanceAlongSpline` _spline_2 _returnvalue_3 "Local") (`SplineComponent.GetLocationAtDistanceAlongSpline` _spline _returnvalue_4 "Local") (`SplineComponent.GetTangentAtDistanceAlongSpline` _spline _returnvalue_4 "Local") true))))))

(fn `UserConstructionScript`
  (`self.GenerateSplineMesh`))